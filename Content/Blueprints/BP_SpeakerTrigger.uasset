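; Interactable speaker trigger that plays a scripted conversation between Kiara and an anonymous voice, then spawns four colored books in the level.
; Box overlap begin and end show and hide the WInteract prompt.
; Interact fires once, requires the overlapping actor to be BP_ThirdPersonCharacter, and sequences 2D dialogue lines with hard-coded delays.
; After the last line starts, it spawns the books at fixed transforms and destroys itself.
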(event `self.Box.OnComponentEndOverlap`
  (params (OverlappedComponent :type "PrimitiveComponent Object Reference") (OtherActor :type "Actor Object Reference") (OtherComp :type "PrimitiveComponent Object Reference") (OtherBodyIndex :type Integer))
  (`SceneComponent.SetVisibility` (`self.W_Interact`) false false))

(event `self.Box.OnComponentBeginOverlap`
  (params (OverlappedComponent :type "PrimitiveComponent Object Reference") (OtherActor :type "Actor Object Reference") (OtherComp :type "PrimitiveComponent Object Reference") (OtherBodyIndex :type Integer) (bFromSweep :type Boolean) (SweepResult :type "HitResult Structure (by ref)"))
  (`SceneComponent.SetVisibility` (`self.W_Interact`) true false :!label _label))

(event `/Game/Blueprints/InteractInterface.Interact`
  (`/Engine/EditorBlueprintResources/StandardMacros.DoOnce` false
    (:`Completed`
      (cast `/Game/ThirdPerson/Blueprints/BP_ThirdPersonCharacter` (stale `self.Box.OnComponentBeginOverlap` OtherActor))
      (`|ExecutionSequence`
        (:`then_0`
          (goto _label))
        (:`then_1`
          (`GameplayStatics.PlayDialogue2D` (`self.Kiara10`) (make `DialogueContext` (`self.KiaraVoice`) (`|MakeArray` (`self.KiaraVoice`))))
          (`KismetSystemLibrary.Delay` 8.0)
          (`GameplayStatics.PlayDialogue2D` (`self.Anonymous1`) (make `DialogueContext` (`self.AnonymousVoice`) (`|MakeArray` (`self.AnonymousVoice`))))
          (`KismetSystemLibrary.Delay` 5.0)
          (`GameplayStatics.PlayDialogue2D` (`self.Kiara11`) (make `DialogueContext` (`self.KiaraVoice`) (`|MakeArray` (`self.KiaraVoice`))))
          (`KismetSystemLibrary.Delay` 4.0)
          (`GameplayStatics.PlayDialogue2D` (`self.Anonymous2`) (make `DialogueContext` (`self.AnonymousVoice`) (`|MakeArray` (`self.AnonymousVoice`))))
          (`KismetSystemLibrary.Delay` 8.0)
          (`GameplayStatics.PlayDialogue2D` (`self.Kiara12`) (make `DialogueContext` (`self.KiaraVoice`) (`|MakeArray` (`self.KiaraVoice`))))
          (`KismetSystemLibrary.Delay` 3.5)
          (`GameplayStatics.PlayDialogue2D` (`self.Anonymous3`) (make `DialogueContext` (`self.AnonymousVoice`) (`|MakeArray` (`self.AnonymousVoice`))))
          (`KismetSystemLibrary.Delay` 13.5)
          (`GameplayStatics.PlayDialogue2D` (`self.Kiara13`) (make `DialogueContext` (`self.KiaraVoice`) (`|MakeArray` (`self.KiaraVoice`))))
          (`KismetSystemLibrary.Delay` 4.0)
          (`GameplayStatics.PlayDialogue2D` (`self.Anonymous4`) (make `DialogueContext` (`self.AnonymousVoice`) (`|MakeArray` (`self.AnonymousVoice`))))
          (`KismetSystemLibrary.Delay` 9.0)
          (`GameplayStatics.PlayDialogue2D` (`self.Kiara14`) (make `DialogueContext` (`self.KiaraVoice`) (`|MakeArray` (`self.KiaraVoice`))))
          (`KismetSystemLibrary.Delay` 8.5)
          (`GameplayStatics.PlayDialogue2D` (`self.Anonymous5`) (make `DialogueContext` (`self.AnonymousVoice`) (`|MakeArray` (`self.AnonymousVoice`))))
          (`KismetSystemLibrary.Delay` 7.5)
          (`GameplayStatics.PlayDialogue2D` (`self.Kiara15`) (make `DialogueContext` (`self.KiaraVoice`) (`|MakeArray` (`self.KiaraVoice`))))
          (`KismetSystemLibrary.Delay` 2.0)
          (`GameplayStatics.PlayDialogue2D` (`self.Anonymous6`) (make `DialogueContext` (`self.AnonymousVoice`) (`|MakeArray` (`self.AnonymousVoice`))))
          (`KismetSystemLibrary.Delay` 4.5)
          (`GameplayStatics.PlayDialogue2D` (`self.Kiara16`) (make `DialogueContext` (`self.KiaraVoice`) (`|MakeArray` (`self.KiaraVoice`))))
          (`|ExecutionSequence`
            (:`then_0`
              (`|SpawnActorFromClass` "/Game/Blueprints/BP_BlueBook.BP_BlueBook_C" (`KismetMathLibrary.MakeTransform` (-1945.0 131.0 86.0) (struct :`Yaw` 90.0 :`Roll` 180.0) (2.0 2.0 2.0)) "Undefined" "MultiplyWithRoot" null null))
            (:`then_1`
              (`|SpawnActorFromClass` "/Game/Blueprints/BP_GreenBook.BP_GreenBook_C" (`KismetMathLibrary.MakeTransform` (-1284.0 -755.0 10.0) (struct :`Yaw` 140.0) (2.25 2.25 2.25)) "Undefined" "MultiplyWithRoot" null null))
            (:`then_2`
              (`|SpawnActorFromClass` "/Game/Blueprints/BP_OrangeBook.BP_OrangeBook_C" (`KismetMathLibrary.MakeTransform` (-1132.0 -479.0 75.0) (struct :`Yaw` 110.0) (1.96875 1.96875 1.96875)) "Undefined" "MultiplyWithRoot" null null))
            (:`then_3`
              (`|SpawnActorFromClass` "/Game/Blueprints/BP_PinkBook.BP_PinkBook_C" (`KismetMathLibrary.MakeTransform` (-2242.0 60.0 105.7) (struct :`Yaw` 110.0)) "Undefined" "MultiplyWithRoot" null null))
            (:`then_4`
              (`self.K2_DestroyActor`))))))))

(fn `UserConstructionScript`)