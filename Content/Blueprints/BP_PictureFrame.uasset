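; BP_PictureFrame is an interactable picture frame that plays two Kiara dialogue lines.
; A box overlap shows and hides the WInteract prompt.
; Interact fires once, casts the begin-overlap actor to BP_ThirdPersonCharacter and sets the prompt visible again.
; It then plays Kiara3 targeted at the player's voice, followed after a fixed delay by Kiara4 targeted at its own voice.
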(event `self.Box.OnComponentEndOverlap`
  (params (OverlappedComponent :type "PrimitiveComponent Object Reference") (OtherActor :type "Actor Object Reference") (OtherComp :type "PrimitiveComponent Object Reference") (OtherBodyIndex :type Integer))
  (`SceneComponent.SetVisibility` (`self.W_Interact`) false false))

(event `self.Box.OnComponentBeginOverlap`
  (params (OverlappedComponent :type "PrimitiveComponent Object Reference") (OtherActor :type "Actor Object Reference") (OtherComp :type "PrimitiveComponent Object Reference") (OtherBodyIndex :type Integer) (bFromSweep :type Boolean) (SweepResult :type "HitResult Structure (by ref)"))
  (`SceneComponent.SetVisibility` (`self.W_Interact`) true false :!label _label))

(event `/Game/Blueprints/InteractInterface.Interact`
  (`/Engine/EditorBlueprintResources/StandardMacros.DoOnce` false
    (:`Completed`
      (bind _asbp_third_person_character (cast `/Game/ThirdPerson/Blueprints/BP_ThirdPersonCharacter` (stale `self.Box.OnComponentBeginOverlap` OtherActor)))
      (`|ExecutionSequence`
        (:`then_0`
          (goto _label))
        (:`then_1`
          (`GameplayStatics.PlayDialogue2D` (`self.Kiara3`) (make `DialogueContext` (`self.DialogueVoice`) (`|MakeArray` (`/Game/ThirdPerson/Blueprints/BP_ThirdPersonCharacter.DialogueVoice` _asbp_third_person_character))))
          (`KismetSystemLibrary.Delay` 6.0)
          (`GameplayStatics.PlayDialogue2D` (`self.Kiara4`) (make `DialogueContext` (`self.DialogueVoice`) (`|MakeArray` (`self.DialogueVoice`)))))))))

(fn `UserConstructionScript`)