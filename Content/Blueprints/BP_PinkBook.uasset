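; BP_PinkBook is an interactable collectible book that shows a prompt widget while something overlaps its sphere.
; Its one-shot Interact event casts the overlapping actor to the third-person character, increments ItemsCollected and spawns BP_PinkBookTrigger at a hardcoded transform.
; It then plays a recorded Kiara and Kyla conversation, sequenced with fixed delays and a radio beep, before destroying itself.
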(event `self.Sphere.OnComponentEndOverlap`
  (params (OverlappedComponent :type "PrimitiveComponent Object Reference") (OtherActor :type "Actor Object Reference") (OtherComp :type "PrimitiveComponent Object Reference") (OtherBodyIndex :type Integer))
  (`SceneComponent.SetVisibility` (`self.W_Interact`) false false))

(event `self.Sphere.OnComponentBeginOverlap`
  (params (OverlappedComponent :type "PrimitiveComponent Object Reference") (OtherActor :type "Actor Object Reference") (OtherComp :type "PrimitiveComponent Object Reference") (OtherBodyIndex :type Integer) (bFromSweep :type Boolean) (SweepResult :type "HitResult Structure (by ref)"))
  (`SceneComponent.SetVisibility` (`self.W_Interact`) true false :!label _label))

(event `/Game/Blueprints/InteractInterface.Interact`
  (`/Engine/EditorBlueprintResources/StandardMacros.DoOnce` false
    (:`Completed`
      (`|ExecutionSequence`
        (:`then_0`
          (bind _asbp_third_person_character (cast `/Game/ThirdPerson/Blueprints/BP_ThirdPersonCharacter` (stale `self.Sphere.OnComponentBeginOverlap` OtherActor)))
          (`|ExecutionSequence`
            (:`then_0`
              (goto _label))
            (:`then_1`
              (bind _result (`/Engine/EditorBlueprintResources/StandardMacros.IncrementInt` (`/Game/ThirdPerson/Blueprints/BP_ThirdPersonCharacter.ItemsCollected` _asbp_third_person_character))
                (:`  `
                  (set `/Game/ThirdPerson/Blueprints/BP_ThirdPersonCharacter.ItemsCollected` _result _asbp_third_person_character)
                  (`|SpawnActorFromClass` "/Game/Blueprints/BP_PinkBookTrigger.BP_PinkBookTrigger_C" (`KismetMathLibrary.MakeTransform` (-887.0 -1115.0 209.0) (struct) (2.15625 2.09375 1.0)) "Undefined" "MultiplyWithRoot" null null))))))
        (:`then_1`
          (`GameplayStatics.PlayDialogue2D` (`self.KiaraRecordingIntro`) (make `DialogueContext` (`self.KiaraVoice`) (`|MakeArray` (`self.KiaraVoice`))))
          (`KismetSystemLibrary.Delay` 6.0)
          (`GameplayStatics.PlayDialogue2D` (`self.KylaRecordingShort`) (make `DialogueContext` (`self.KylaVoice`) (`|MakeArray` (`self.KylaVoice`))))
          (`KismetSystemLibrary.Delay` 2.0)
          (`GameplayStatics.PlayDialogue2D` (`self.KiaraRecordingStart`) (make `DialogueContext` (`self.KiaraVoice`) (`|MakeArray` (`self.KiaraVoice`))))
          (`KismetSystemLibrary.Delay` 2.0)
          (`GameplayStatics.PlayDialogue2D` (`self.KylaRecordingLong`) (make `DialogueContext` (`self.KylaVoice`) (`|MakeArray` (`self.KylaVoice`))))
          (`KismetSystemLibrary.Delay` 16.0)
          (`GameplayStatics.PlaySound2D` "/Game/Audio/259710__alienxxx__radio_beep.259710__alienxxx__radio_beep" 1.0 1.0 0.0 null null)
          (`KismetSystemLibrary.Delay` 1.5)
          (`GameplayStatics.PlayDialogue2D` (`self.KiaraRecordingEnd`) (make `DialogueContext` (`self.KiaraVoice`) (`|MakeArray` (`self.KiaraVoice`))))
          (`self.K2_DestroyActor`))))))

(fn `UserConstructionScript`)