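; BP_Door is an interactable door whose opening leads to the game's end screen.
; An overlap box toggles an interact prompt, and Interact flip-flops a timeline that yaws the mesh between 0 and 90 degrees.
; The timeline's Update, in either direction, also fires a sound every tick, then delayed Kiara dialogue and the W_End widget with UI-only input and cursor.
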(event `/Game/Blueprints/InteractInterface.Interact`
  (bind _returnvalue (`GameplayStatics.GetPlayerController` 0))
  (`/Engine/EditorBlueprintResources/StandardMacros.FlipFlop`
    (:`A`
      (bind (_direction _door_track) (`Timeline|open/Close door timeline` :!label _label)
        (:`Update`
          (`SceneComponent.K2_SetRelativeRotation` (`self.StaticMesh`) (`KismetMathLibrary.MakeRotator` 0.0 0.0 (`KismetMathLibrary.Lerp` 0.0 90.0 _door_track)) false false)
          (`GameplayStatics.PlaySound2D` "/Game/Audio/524612__clearwavsound__neck-bone-snap.524612__clearwavsound__neck-bone-snap" 1.0 1.0 0.0 null null)
          (`KismetSystemLibrary.Delay` 1.0)
          (`GameplayStatics.PlayDialogue2D` (`self.Kiara20`) (make `DialogueContext` (`self.KiaraVoice`) (`|MakeArray` (`self.KiaraVoice`))))
          (`KismetSystemLibrary.Delay` 8.0)
          (bind _returnvalue_2 (`|CreateWidget` "/Game/WidgetsUI/W_End.W_End_C"))
          (`UserWidget.AddToViewport` _returnvalue_2 0)
          (`WidgetBlueprintLibrary.SetInputMode_UIOnlyEx` _returnvalue null)
          (set `PlayerController.bShowMouseCursor` true _returnvalue))))
    (:`B`
      (goto _label :!via `Reverse`))))

(event `self.Box.OnComponentBeginOverlap`
  (params (OverlappedComponent :type "PrimitiveComponent Object Reference") (OtherActor :type "Actor Object Reference") (OtherComp :type "PrimitiveComponent Object Reference") (OtherBodyIndex :type Integer) (bFromSweep :type Boolean) (SweepResult :type "HitResult Structure (by ref)"))
  (cast `/Game/ThirdPerson/Blueprints/BP_ThirdPersonCharacter` OtherActor)
  (`SceneComponent.SetVisibility` (`self.W_Interact`) true false))

(event `self.Box.OnComponentEndOverlap`
  (params (OverlappedComponent :type "PrimitiveComponent Object Reference") (OtherActor :type "Actor Object Reference") (OtherComp :type "PrimitiveComponent Object Reference") (OtherBodyIndex :type Integer))
  (`SceneComponent.SetVisibility` (`self.W_Interact`) false false))

(fn `UserConstructionScript`)