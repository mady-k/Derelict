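; BP_BlueBook is an interactable book that shows a prompt widget while its sphere is overlapped and starts a Kiara photo story beat.
; Interact runs once, casts the overlapping actor to BP_ThirdPersonCharacter, increments ItemsCollected and spawns BP_BlueBookTrigger at a hardcoded transform.
; A delayed sequence then plays Kiara's dialogue around opening W_KylaPhoto with UI-only input and a mouse cursor, and finally destroys the book.
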(event `self.Sphere.OnComponentEndOverlap`
  (params (OverlappedComponent :type "PrimitiveComponent Object Reference") (OtherActor :type "Actor Object Reference") (OtherComp :type "PrimitiveComponent Object Reference") (OtherBodyIndex :type Integer))
  (`SceneComponent.SetVisibility` (`self.W_Interact`) false false))

(event `self.Sphere.OnComponentBeginOverlap`
  (params (OverlappedComponent :type "PrimitiveComponent Object Reference") (OtherActor :type "Actor Object Reference") (OtherComp :type "PrimitiveComponent Object Reference") (OtherBodyIndex :type Integer) (bFromSweep :type Boolean) (SweepResult :type "HitResult Structure (by ref)"))
  (`SceneComponent.SetVisibility` (`self.W_Interact`) true false :!label _label))

(event `/Game/Blueprints/InteractInterface.Interact`
  (bind _returnvalue (`GameplayStatics.GetPlayerController` 0))
  (`/Engine/EditorBlueprintResources/StandardMacros.DoOnce` false
    (:`Completed`
      (`|ExecutionSequence`
        (:`then_0`
          (bind _asbp_third_person_character (cast `/Game/ThirdPerson/Blueprints/BP_ThirdPersonCharacter` (stale `self.Sphere.OnComponentBeginOverlap` OtherActor)))
          (`|ExecutionSequence`
            (:`then_0`
              (goto _label))
            (:`then_1`
              (bind _result (`/Engine/EditorBlueprintResources/StandardMacros.IncrementInt` (`/Game/ThirdPerson/Blueprints/BP_ThirdPersonCharacter.ItemsCollected` _asbp_third_person_character))
                (:`  `
                  (set `/Game/ThirdPerson/Blueprints/BP_ThirdPersonCharacter.ItemsCollected` _result _asbp_third_person_character)
                  (`|ExecutionSequence`
                    (:`then_0`
                      (`|SpawnActorFromClass` "/Game/Blueprints/BP_BlueBookTrigger.BP_BlueBookTrigger_C" (`KismetMathLibrary.MakeTransform` (-847.0 -1116.0 114.0) (struct) (2.15625 2.09375 1.0)) "Undefined" "MultiplyWithRoot" null null))
                    (:`then_1`
                      (`KismetSystemLibrary.Delay` 1.0)
                      (`GameplayStatics.PlayDialogue2D` (`self.KiaraPhotoIntro`) (make `DialogueContext` (`self.KiaraVoice`) (`|MakeArray` (`self.KiaraVoice`))))
                      (`KismetSystemLibrary.Delay` 3.0)
                      (`WidgetBlueprintLibrary.SetInputMode_UIOnlyEx` _returnvalue null)
                      (set `PlayerController.bShowMouseCursor` true _returnvalue)
                      (bind _returnvalue_2 (`|CreateWidget` "/Game/WidgetsUI/W_KylaPhoto.W_KylaPhoto_C"))
                      (`UserWidget.AddToViewport` _returnvalue_2 0)
                      (`KismetSystemLibrary.Delay` 2.0)
                      (`GameplayStatics.PlayDialogue2D` (`self.KiaraPhoto`) (make `DialogueContext` (`self.KiaraVoice`) (`|MakeArray` (`self.KiaraVoice`))))
                      (`KismetSystemLibrary.Delay` 1.0)
                      (`self.K2_DestroyActor`))))))))))))

(fn `UserConstructionScript`)