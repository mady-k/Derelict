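; BP_LockedDoor is a puzzle door that shows an interact widget while the player character is in its box.
; First Interact plays a one-time dialogue and sound sequence, then spawns BP_SpeakerTrigger.
; Interact also checks the character's ItemsCollected for four items, then FlipFlops a rotation timeline open or closed.
; The timeline's Update also drives a delayed dialogue exchange; the door's own item-counting logic is largely disconnected.
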(event `OpenPuzzleDoor`
  (`/Engine/EditorBlueprintResources/StandardMacros.FlipFlop`
    (:`A`
      (bind (_direction _door_rotation) (`Timeline|open door` :!label _label)
        (:`Update`
          (`SceneComponent.K2_SetRelativeRotation` (`self.StaticMesh`) (`KismetMathLibrary.MakeRotator` 0.0 0.0 (`KismetMathLibrary.Lerp` 0.0 90.0 _door_rotation)) false false)
          (`GameplayStatics.PlaySound2D` "/Game/Audio/Hit_Hurt5.Hit_Hurt5" 1.0 1.0 0.0 null null)
          (`KismetSystemLibrary.Delay` 1.0)
          (`GameplayStatics.PlayDialogue2D` (`self.Anonymous7`) (make `DialogueContext` (`self.AnonymousVoice`) (`|MakeArray` (`self.AnonymousVoice`))))
          (`KismetSystemLibrary.Delay` 1.0)
          (`GameplayStatics.PlayDialogue2D` (`self.Kiara17`) (make `DialogueContext` (`self.KiaraVoice`) (`|MakeArray` (`self.KiaraVoice`))))
          (`KismetSystemLibrary.Delay` 1.0)
          (`GameplayStatics.PlayDialogue2D` (`self.Anonymous8`) (make `DialogueContext` (`self.AnonymousVoice`) (`|MakeArray` (`self.AnonymousVoice`))))
          (`KismetSystemLibrary.Delay` 1.0)
          (`GameplayStatics.PlayDialogue2D` (`self.Kiara18`) (make `DialogueContext` (`self.KiaraVoice`) (`|MakeArray` (`self.KiaraVoice`))))
          (`KismetSystemLibrary.Delay` 1.0)
          (`GameplayStatics.PlayDialogue2D` (`self.Anonymous9`) (make `DialogueContext` (`self.AnonymousVoice`) (`|MakeArray` (`self.AnonymousVoice`))))
          (`KismetSystemLibrary.Delay` 1.0)
          (`GameplayStatics.PlayDialogue2D` (`self.Kiara19`) (make `DialogueContext` (`self.KiaraVoice`) (`|MakeArray` (`self.KiaraVoice`)))))))
    (:`B`
      (goto _label :!via `Reverse`))))

(event `Collectitem`
  (bind _returnvalue (`GameplayStatics.GetActorOfClass` "BP_LockedDoor_C")))

(event `OpenDoorCheck`
  (if (>= (`self.CurrentItemsCollected`) 4)
    (`/Engine/EditorBlueprintResources/StandardMacros.DoOnce` false
      (:`Completed`
        (`self.OpenPuzzleDoor`)))))

(event `/Game/Blueprints/InteractInterface.Interact`
  (`|ExecutionSequence`
    (:`then_0`
      (`/Engine/EditorBlueprintResources/StandardMacros.DoOnce` false
        (:`Completed`
          (`GameplayStatics.PlayDialogue2D` (`self.Kiara7`) (make `DialogueContext` (`self.KiaraVoice`) (`|MakeArray` (`self.KiaraVoice`))))
          (`KismetSystemLibrary.Delay` 3.5)
          (`GameplayStatics.PlaySound2D` "/Game/Audio/453972__kyles__door-wood-glass-bang-on-hits.453972__kyles__door-wood-glass-bang-on-hits" 1.0 1.0 0.0 null null)
          (`KismetSystemLibrary.Delay` 2.5)
          (`GameplayStatics.PlayDialogue2D` (`self.Kiara8`) (make `DialogueContext` (`self.KiaraVoice`) (`|MakeArray` (`self.KiaraVoice`))))
          (`KismetSystemLibrary.Delay` 4.5)
          (`GameplayStatics.PlaySound2D` "/Game/Audio/255572__stradie__static.255572__stradie__static" 1.0 1.0 0.0 null null)
          (`KismetSystemLibrary.Delay` 5.0)
          (`GameplayStatics.PlayDialogue2D` (`self.Kiara9`) (make `DialogueContext` (`self.KiaraVoice`) (`|MakeArray` (`self.KiaraVoice`))))
          (`|SpawnActorFromClass` "/Game/Blueprints/BP_SpeakerTrigger.BP_SpeakerTrigger_C" (`KismetMathLibrary.MakeTransform` (-832.0 -340.0 198.0) (struct) (2.125 3.0 6.34375)) "Undefined" "MultiplyWithRoot" null null))))
    (:`then_1`
      (bind _asbp_third_person_character (cast `/Game/ThirdPerson/Blueprints/BP_ThirdPersonCharacter` (`GameplayStatics.GetPlayerCharacter` 0)))
      (if (>= (`/Game/ThirdPerson/Blueprints/BP_ThirdPersonCharacter.ItemsCollected` _asbp_third_person_character) 4)
        (`self.OpenPuzzleDoor`)))))

(event `self.Box.OnComponentBeginOverlap`
  (params (OverlappedComponent :type "PrimitiveComponent Object Reference") (OtherActor :type "Actor Object Reference") (OtherComp :type "PrimitiveComponent Object Reference") (OtherBodyIndex :type Integer) (bFromSweep :type Boolean) (SweepResult :type "HitResult Structure (by ref)"))
  (cast `/Game/ThirdPerson/Blueprints/BP_ThirdPersonCharacter` OtherActor)
  (`SceneComponent.SetVisibility` (`self.W_Interact`) true false))

(event `self.Box.OnComponentEndOverlap`
  (params (OverlappedComponent :type "PrimitiveComponent Object Reference") (OtherActor :type "Actor Object Reference") (OtherComp :type "PrimitiveComponent Object Reference") (OtherBodyIndex :type Integer))
  (`SceneComponent.SetVisibility` (`self.W_Interact`) false false))

(fn `UserConstructionScript`)